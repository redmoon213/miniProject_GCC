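; GC_BP_EnemyBlue is a Geometry Collection actor, apparently the shattering stand-in for a blue enemy.
; Shortly after BeginPlay it wakes the collection's rigid bodies and applies an upward impulse.
; It then applies heavy radial damage around its own location and sets a short lifespan so the debris cleans itself up.
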(event EventBeginPlay
  (Utilities|FlowControl|Delay 0.1)
  (Class|PrimitiveComponent|WakeRigidBody (Variables|Default|GetGeometryCollection) "None")
  (Physics|AddImpulse (Variables|Default|GetGeometryCollection) "0.000000,0.000000,1000.000000" "None" false)
  (Game|Damage|ApplyRadialDamage 5e+03 (Transformation|GetActorLocation) 3e+02 0 0 self 0 false "ECC_Visibility")
  (Actor|SetLifeSpan 2.0))

(event Collision|EventActorBeginOverlap
  (params (OtherActor :type Actor%20Object%20Reference)))

(event EventTick
  (params (DeltaSeconds :type Float%20%28single-precision%29)))

(fn ConstructionScript)